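; BP_Arrow is an arrow projectile that scores hits on BP_Target in a first-person archery setup.
; ArrowShot spawns an arrow at the player pawn along camera rotation and sets its local-space velocity.
; On hit, it maps the struck cylinder component's name to 0–10 points, with misses scoring zero, and plays a sound.
; It then disables collision and sends the points to the player's last-shot widget; GetPoints is a stub.
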(event OnComponentHit(Collision)
  (params (HitComponent :type Primitive%20Component%20Object%20Reference) (OtherActor :type Actor%20Object%20Reference) (OtherComp :type Primitive%20Component%20Object%20Reference) (NormalImpulse :type Vector :default "0, 0, 0") (Hit :type Hit%20Result%20Structure%20%28by%20ref%29))
  (bind _returnvalue (Transformation|GetActorLocation))
  (if (== (Utilities|GetClass OtherActor) "/Game/Classes/BP_Target.BP_Target_C")
    (Development|PrintString "HIT")
    (Audio|PlaySoundatLocation "/Game/Sounds/SW_hit.SW_hit" _returnvalue "0, 0, 0" 1.0 1.0 0.0 0 0 0 0)
    (switch string (Utilities|GetObjectName OtherComp)
      (:Default
        (Variables|Default|SetPointsHit 0 :!label _label))
      (:Cylinder
        (Variables|Default|SetPointsHit 1))
      (:Cylinder_001
        (Variables|Default|SetPointsHit 2))
      (:Cylinder_002
        (Variables|Default|SetPointsHit 3))
      (:Cylinder_003
        (Variables|Default|SetPointsHit 4))
      (:Cylinder_004
        (Variables|Default|SetPointsHit 5))
      (:Cylinder_005
        (Variables|Default|SetPointsHit 6))
      (:Cylinder_006
        (Variables|Default|SetPointsHit 7))
      (:Cylinder_007
        (Variables|Default|SetPointsHit 8))
      (:Cylinder_008
        (Variables|Default|SetPointsHit 9))
      (:Cylinder_009
        (Variables|Default|SetPointsHit 10)))
    (else
      (Development|PrintString "MISSED")
      (Audio|PlaySoundatLocation "/Game/Sounds/SW_miss.SW_miss" _returnvalue "0, 0, 0" 1.0 1.0 0.0 0 0 0 0)
      (goto _label)))
  (Collision|SetCollisionEnabled (Variables|Default|GetCollision) "NoCollision")
  (bind _asbp_first_person_character (Utilities|Casting|CastToBP_FirstPersonCharacter (Game|GetPlayerCharacter 0)))
  (Default|UpdateLastShotPoints (Variables|/Game/FirstPerson/Blueprints/BP_FirstPersonCharacter.BP_FirstPersonCharacter_C|GetLastShotWidget _asbp_first_person_character) (Variables|Default|GetPointsHit)))

(fn ConstructionScript)

(fn ArrowShot
  (bind _returnvalue (Game|SpawnActorfromClass "BP_Arrow_C" (Math|Transform|MakeTransform (Transformation|GetActorLocation (Game|Player|GetPlayerPawn 0)) (Camera|GetCameraRotation (Game|GetPlayerCameraManager 0))) "Undefined" "MultiplyWithRoot" 0 0))
  (Game|Components|ProjectileMovement|SetVelocityinLocalSpace (Variables|BP_Arrow_C|GetProjectileMovement _returnvalue) (Variables|Default|GetVelocity)))

(fn GetPoints
  (params (PointsHit :type Integer))
  (return 0))